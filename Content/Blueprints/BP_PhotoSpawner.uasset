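; BP_PhotoSpawner continually spawns waves of moving targets, apparently subjects for a photo mechanic.
; After BeginPlay, SpawnTarget waits a few random seconds, spawns SpawnCount random TargetList classes, then calls itself to repeat.
; Targets appear scaled up at SpawnHeight, offset by index on either side along Y.
; Side, offset sign, rotation and Y-axis MoveDirection use separate random rolls, so facing and travel can disagree.
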(event `self.ReceiveBeginPlay`
  (`self.SpawnTarget`))

(event `SpawnTarget`
  (bind _returnvalue (`KismetMathLibrary.RandomBool`))
  (bind _targetlist (`self.TargetList`))
  (`KismetSystemLibrary.Delay` (`KismetMathLibrary.RandomFloatInRange` 3.0 5.0))
  (for _index (range (`self.SpawnCount`))
    (bind _returnvalue_2 (`|SpawnActorFromClass` (`|GetArrayItem` _targetlist (`KismetMathLibrary.RandomIntegerInRange` 0 (`KismetArrayLibrary.Array_LastIndex` _targetlist))) (`KismetMathLibrary.MakeTransform` (`KismetMathLibrary.MakeVector` 1500.0 (+ (* _index (select `bool` _returnvalue :`false` -150.0 :`true` 150.0)) (select `bool` _returnvalue :`false` -2000.0 :`true` 2000.0)) (`self.SpawnHeight`)) (select `bool` _returnvalue :`true` (struct :`Yaw` 180.0) :!type "Rotator Structure") (3.0 3.0 3.0)) "AlwaysSpawn" "MultiplyWithRoot" null null))
    (set `/Game/Blueprints/BP_Target_Base.MoveDirection` (select `bool` _returnvalue :`false` (0.0 1.0 0.0) :`true` (0.0 -1.0 0.0) :!type "Vector Structure") _returnvalue_2))
  (`self.SpawnTarget`))

(fn `UserConstructionScript`)