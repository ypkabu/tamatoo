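; Enemy actor that travels via an InterpToMovement component and can pause to play a throw attack animation.
; Tick feeds the AnimBP_Enemy SideSpeed from the sign of delta time, so it is effectively a fixed value rather than measured velocity.
; PauseForThrow disables the movement component's tick and plays the attack montage, followed by a delay that leads nowhere.
; ResumeMovement cuts the montage without blending and re-enables that tick.
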(event `self.ReceiveTick`
  (params (DeltaSeconds :type "Float (single-precision)"))
  (bind _asanim_bp_enemy (cast `/Game/Blueprints/AnimBP_Enemy` (`SkeletalMeshComponent.GetAnimInstance` (`self.SkeletalMesh`))))
  (set `/Game/Blueprints/AnimBP_Enemy.SideSpeed` (* (`KismetMathLibrary.SignOfFloat` DeltaSeconds) 500.0) _asanim_bp_enemy))

(event `PauseForThrow`
  (`ActorComponent.SetComponentTickEnabled` (`self.InterpToMovement`) false)
  (`|PlayMontage` (`self.SkeletalMesh`) "/Game/RPGHeroSquad/Animation/TinyHero/Anim_Attack02_Montage.Anim_Attack02_Montage"
    (:`then`
      (`KismetSystemLibrary.Delay` 1.0))))

(event `ResumeMovement`
  (`AnimInstance.Montage_Stop` (`SkeletalMeshComponent.GetAnimInstance` (`self.SkeletalMesh`)) 0.0 "/Game/RPGHeroSquad/Animation/TinyHero/Anim_Attack02_Montage.Anim_Attack02_Montage")
  (`ActorComponent.SetComponentTickEnabled` (`self.InterpToMovement`) true))

(fn `UserConstructionScript`)