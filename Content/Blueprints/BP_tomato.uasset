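; BP_tomato is a short-lived sprite projectile that splatters on the player's view.
; BeginPlay applies its Speed to the projectile movement, and Tick yaw-billboards the sprite toward the camera.
; A per-tick camera distance check replaces overlap detection: when close, it spawns a jittered BP_Dirt splat, plays a squish, shakes the camera, resets the player's ComboCount and destroys itself.
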(event `self.ReceiveTick`
  (params (DeltaSeconds :type "Float (single-precision)"))
  (`SceneComponent.K2_SetWorldRotation` (`self.PaperSprite`) (`KismetMathLibrary.MakeRotator` 0.0 0.0 (+ (.yaw (`KismetMathLibrary.FindLookAtRotation` (`self.K2_GetActorLocation`) (`PlayerCameraManager.GetCameraLocation` (`GameplayStatics.GetPlayerCameraManager` 0)))) 90.0)) false false)
  (`self.HitSplash`))

(event `self.ReceiveBeginPlay`
  (bind _projectilemovement (`self.ProjectileMovement`))
  (bind _speed (`self.Speed`))
  (set `ProjectileMovementComponent.InitialSpeed` _speed _projectilemovement)
  (set `ProjectileMovementComponent.MaxSpeed` _speed _projectilemovement)
  (`self.SetLifeSpan` 2.0))

(event `HitSplash`
  (bind _returnvalue (`GameplayStatics.GetPlayerCameraManager` 0))
  (bind _returnvalue_2 (`self.K2_GetActorLocation`))
  (if (< (`KismetMathLibrary.Vector_Distance` (`PlayerCameraManager.GetCameraLocation` _returnvalue) _returnvalue_2) 8.0)
    (`|SpawnActorFromClass` "/Game/Blueprints/BP_Dirt.BP_Dirt_C" (`KismetMathLibrary.MakeTransform` (+ _returnvalue_2 (`KismetMathLibrary.MakeVector` 0.0 (`KismetMathLibrary.RandomFloatInRange` -1.0 1.0) (`KismetMathLibrary.RandomFloatInRange` -1.0 1.0))) (`KismetMathLibrary.ComposeRotators` (`PlayerCameraManager.GetCameraRotation` _returnvalue) (struct :`Yaw` 90.0))) "Undefined" "MultiplyWithRoot" null null)
    (`GameplayStatics.PlaySound2D` "/Game/Sounds/Squish_Cue.Squish_Cue" 1.0 1.0 0.0 null null)
    (`PlayerCameraManager.StartCameraShake` :`self` (`GameplayStatics.GetPlayerCameraManager` 0) :`ShakeClass` "/Game/Blueprints/CS_Shake.CS_Shake_C")
    (bind _asbp_first_person_character (cast `/Game/FirstPerson/Blueprints/BP_FirstPersonCharacter` (`GameplayStatics.GetPlayerCharacter` 0)))
    (set `/Game/FirstPerson/Blueprints/BP_FirstPersonCharacter.ComboCount` 0.0 _asbp_first_person_character)
    (`self.K2_DestroyActor`)))

(fn `UserConstructionScript`)