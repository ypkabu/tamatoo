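; BP_Tomato_Slider is a tomato actor that flies a curved slider path toward the first-person player's HomingTargetMark.
; On BeginPlay it stores its start location and plays a timeline that lerps it to the mark's current position each update.
; A second timeline curve adds sideways bend along the mark's right vector.
; Movement is unswept SetActorLocation; ProjectileMovement and a sine-offset fragment are unused, and no hit logic exists in the graph.
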(event `self.ReceiveBeginPlay`
  (`parent.ReceiveBeginPlay`)
  (bind _asbp_first_person_character (cast `/Game/FirstPerson/Blueprints/BP_FirstPersonCharacter` (`GameplayStatics.GetPlayerCharacter` 0)))
  (set `self.StartLocation` (`self.K2_GetActorLocation`))
  (bind (_direction _forwardalpha _curvealpha) (`Timeline|SliderTimeline`)
    (:`Update`
      (bind _homingtargetmark (`/Game/FirstPerson/Blueprints/BP_FirstPersonCharacter.HomingTargetMark` _asbp_first_person_character))
      (`self.K2_SetActorLocation` (+ (`KismetMathLibrary.VLerp` (`self.StartLocation`) (- (`SceneComponent.K2_GetComponentLocation` _homingtargetmark) (0.0 0.0 0.0)) _forwardalpha) (* (* (`SceneComponent.GetRightVector` _homingtargetmark) 50.0) _curvealpha))))))

(event `self.ReceiveTick`
  (params (DeltaSeconds :type "Float (single-precision)"))
  (`parent.ReceiveTick` DeltaSeconds))

(fn `UserConstructionScript`
  (`parent.UserConstructionScript`))