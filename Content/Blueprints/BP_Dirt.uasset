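; BP_Dirt is a wipeable dirt spot, shown as a Paper2D sprite, that fades as it is cleaned.
; TakeWipe subtracts the wipe amount from DirtHealth and maps the remaining health to the sprite's alpha.
; When health runs out, it calls RequestSqueak on the player's BP_FirstPersonCharacter and destroys itself.
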(event `TakeWipe`
  (params (WipeAmount :type "Float (double-precision)"))
  (bind _output_get (set `self.DirtHealth` (- (`self.DirtHealth`) WipeAmount)))
  (`PaperSpriteComponent.SetSpriteColor` (`self.PaperSprite`) (make `LinearColor` 1.0 1.0 1.0 (`KismetMathLibrary.MapRangeClamped` (`self.DirtHealth`) 0.0 100.0 0.0 1.0)))
  (if (<= _output_get 0.0)
    (bind _asbp_first_person_character (cast `/Game/FirstPerson/Blueprints/BP_FirstPersonCharacter` (`GameplayStatics.GetPlayerCharacter` 0)))
    (`/Game/FirstPerson/Blueprints/BP_FirstPersonCharacter.RequestSqueak` _asbp_first_person_character)
    (`self.K2_DestroyActor`)))

(fn `UserConstructionScript`)