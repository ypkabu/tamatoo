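; Tomato spawner actor that creates the game UI at BeginPlay and repeatedly spawns tomatoes in front of the player's camera.
; A self-calling SpawnLoop waits a random delay, then spawns a batch of randomly chosen straight, parabola or slider tomato classes with random offsets, camera-facing rotation and random speed.
; The UI widget's NowTime/MaxQuota ratio drives difficulty, shortening delays and growing batches as it rises.
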(event `self.ReceiveBeginPlay`
  (bind _returnvalue (`|CreateWidget` "/Game/UI/WBP_GameUI.WBP_GameUI_C"))
  (bind _output_get (set `self.NewVar` _returnvalue))
  (`UserWidget.AddToViewport` _output_get 0)
  (`self.SpawnLoop`))

(event `SpawnLoop`
  (bind _returnvalue (`GameplayStatics.GetPlayerCameraManager` 0))
  (bind _returnvalue_2 (`GameplayStatics.GetPlayerCameraManager` 0))
  (bind _newvar (`self.NewVar`))
  (bind _returnvalue_3 (`PlayerCameraManager.GetCameraLocation` _returnvalue_2))
  (bind _returnvalue_4 (/ (`/Game/UI/WBP_GameUI.NowTime` _newvar) (`/Game/UI/WBP_GameUI.MaxQuota` _newvar)))
  (bind _returnvalue_5 (+ (+ _returnvalue_3 (* (`self.GetActorForwardVector` _returnvalue_2) 100.0)) (`KismetMathLibrary.MakeVector` 0.0 (`KismetMathLibrary.RandomFloatInRange` -50.0 50.0) (`KismetMathLibrary.RandomFloatInRange` -20.0 20.0))))
  (`KismetSystemLibrary.Delay` (`KismetMathLibrary.RandomFloatInRange` (`KismetMathLibrary.MapRangeClamped` _returnvalue_4 0.0 1.0 1.5 0.5) (`KismetMathLibrary.MapRangeClamped` _returnvalue_4 0.0 1.0 3.0 1.0)))
  (for _ (range 1 (+ (`KismetMathLibrary.FTrunc` (`KismetMathLibrary.MapRangeClamped` _returnvalue_4 0.0 1.0 1.0 3.7)) 1))
    (set `self.Random` (`KismetMathLibrary.RandomIntegerInRange` 0 2))
    (bind _returnvalue_6 (`|SpawnActorFromClass` (select `int` (`self.Random`) :`0` "/Game/Blueprints/BP_tomato.BP_tomato_C" :`1` "/Game/Blueprints/BP_Tomato_Parabola.BP_Tomato_Parabola_C" :`2` "/Game/Blueprints/BP_Tomato_Slider.BP_Tomato_Slider_C" :!type "Actor Class Reference") (`KismetMathLibrary.MakeTransform` (select `int` (`self.Random`) :`0` _returnvalue_5 :`1` (+ (+ (`PlayerCameraManager.GetCameraLocation` _returnvalue) (* (`self.GetActorForwardVector` _returnvalue) 100.0)) (`KismetMathLibrary.MakeVector` 0.0 (`KismetMathLibrary.RandomFloatInRange` -30.0 30.0))) :`2` _returnvalue_5) (`KismetMathLibrary.FindLookAtRotation` _returnvalue_5 _returnvalue_3) (0.4 0.4 0.4)) "AlwaysSpawn" "MultiplyWithRoot" null null))
    (bind _asbp_tomato (cast `/Game/Blueprints/BP_tomato` _returnvalue_6))
    (set `/Game/Blueprints/BP_tomato.Speed` (`KismetMathLibrary.RandomFloatInRange` 40.0 70.0) _asbp_tomato))
  (`self.SpawnLoop`))

(fn `UserConstructionScript`)